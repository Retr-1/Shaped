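; Game instance holding run state across levels: XP and skills, money, ammo stack, base health and cycle count.
; Skills unlock with XP once prerequisites are met; money comes from selling bullets and pays for wildcards and base repairs, with events broadcasting changes.
; Fired bullets are recorded, then reinserted at stack index 0 when Fight returns to Factory.
; Zero base health shows the game-over screen; starting from the main menu resets the run.
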(fn AddXP
  (params (Amount :type Integer))
  (Variables|Default|SetPlayerXP (+ Amount (Variables|Default|GetPlayerXP)))
  (Default|CallPlayerXPUpdated self))

(fn UnlockSkill
  (params (ID :type E_Skills%20Enum :default "NewEnumerator0"))
  (bind _skillsmap (Variables|Default|GetSkillsMap))
  (bind _value (Utilities|Map|Find _skillsmap ID))
  (if (and (Utilities|Set|Contains (Variables|Default|GetAvaibleSkills) ID) (<= (.cost _value) (Variables|Default|GetPlayerXP)))
    (Variables|Default|SetPlayerXP (- (Variables|Default|GetPlayerXP) (.cost _value)))
    (Utilities|Set|Add (Variables|Default|GetUnlockedSkills) ID)
    (Utilities|Set|Remove (Variables|Default|GetAvaibleSkills) ID)
    (CallFunction|UpdateAvaibleSkills)
    (Default|CallPlayerXPUpdated self)
    (Default|CallSkillsUpdated)))

(fn UpdateAvaibleSkills
  (bind _enumvalue (|ForEachE_Skills)
    (:LoopBody
      (if (not (Utilities|Set|Contains (Variables|Default|GetUnlockedSkills) _enumvalue))
        (LocalVariables|SetHasAllRequisites true)
        (bind _valuepin (Utilities|Set|ForEachLoop(Set) (.prerequisites (.Value (Utilities|Map|Find (Variables|Default|GetSkillsMap) _enumvalue))))
          (:then
            (LocalVariables|SetHasAllRequisites (and (Utilities|Set|Contains (Variables|Default|GetUnlockedSkills) _valuepin) (LocalVariables|GetHasAllRequisites))))
          (:CompletedPin
            (if (LocalVariables|GetHasAllRequisites)
              (Utilities|Set|Add (Variables|Default|GetAvaibleSkills) _enumvalue))))))))

(fn SellTopBullet
  (if (not (Utilities|Array|IsEmpty (Variables|Default|GetAmmoStack)))
    (Class|ShapedGameInstance|PopAmmo)
    (Variables|Default|SetMoney (+ (Variables|Default|GetMoneyGainPerBullet) (Variables|Default|GetMoney)))
    (Default|CallMoneyUpdated self)))

(fn BuyWildcardBullet
  (if (>= (Variables|Default|GetMoney) (Variables|Default|GetWildardBulletBuyCost))
    (Class|ShapedGameInstance|PushAmmo "www")
    (Variables|Default|SetMoney (- (Variables|Default|GetMoney) (Variables|Default|GetWildardBulletBuyCost)))
    (Default|CallMoneyUpdated self)))

(fn RepairBase
  (if (and (>= (Variables|Default|GetMoney) (Variables|Default|GetRepairBaseCost)) (< (Variables|Default|GetBaseHealth) (Variables|Default|GetBaseMaxHealth)))
    (Variables|Default|SetBaseHealth (Math|Float|Clamp(Float) (+ (Variables|Default|GetBaseHealth) (Variables|Default|GetRepairBaseAmount)) 0.0 (Variables|Default|GetBaseMaxHealth)))
    (Variables|Default|SetMoney (- (Variables|Default|GetMoney) (Variables|Default|GetRepairBaseCost)))
    (Default|CallMoneyUpdated self)
    (Default|CallBaseHealthUpdated self)))

(fn ApplyDamagetoBase
  (params (Damage :type Float%20%28double-precision%29))
  (Variables|Default|SetBaseHealth (- (Variables|Default|GetBaseHealth) Damage))
  (Default|CallBaseHealthUpdated self)
  (if (<= (Variables|Default|GetBaseHealth) 0.0)
    (CallFunction|EndGame)))

(fn MovefromFighttoFactory
  (if (not (Variables|Default|GetGameOver))
    (Variables|Default|SetCycle (+ (Variables|Default|GetCycle) 1))
    (for _array_element (Variables|Default|GetFiredBullets)
      (Utilities|Array|Insert (Variables|Default|GetAmmoStack) _array_element))
    (Utilities|Array|Clear (Variables|Default|GetFiredBullets))
    (Class|ShapedGameInstance|BroadcastAmmoStackChanged)
    (Game|OpenLevel(byName) "Factory")))

(fn FireAmmo
  (bind _outammoid (Class|ShapedGameInstance|PopAmmo))
  (Utilities|Array|Add (Variables|Default|GetFiredBullets) _outammoid)
  (return _outammoid))

(fn EndGame
  (bind _returnvalue (Game|GetPlayerController 0))
  (Input|SetInputModeUIOnly _returnvalue 0 "DoNotLock" false)
  (Variables|/Script/Engine.PlayerController|SetbShowMouseCursor _returnvalue true)
  (bind _returnvalue_2 (Game|ConstructObjectfromClass "/Game/Blueprints/Widgets/WBP_GameOver.WBP_GameOver_C" (Variables|Default|GetCycle)))
  (UserInterface|Viewport|AddtoViewport _returnvalue_2 0)
  (Variables|Default|SetGameOver true))

(fn Reset
  (Variables|Default|SetPlayerXP 0)
  (Utilities|Set|Clear (Variables|Default|GetAvaibleSkills))
  (Utilities|Set|Clear (Variables|Default|GetUnlockedSkills))
  (CallFunction|UpdateAvaibleSkills)
  (Variables|Default|SetMoney 0)
  (Variables|Default|SetBaseHealth (Variables|Default|GetBaseMaxHealth))
  (Variables|Default|SetCycle 0)
  (Utilities|Array|Clear (Variables|Default|GetFiredBullets))
  (Utilities|Array|Clear (Variables|Default|GetAmmoStack))
  (Variables|Default|SetGameOver false))

(fn MovefromMainMenutoFactory
  (CallFunction|Reset)
  (Game|OpenLevel(byName) "Factory"))