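; StateTree task that turns an enemy actor in place by a random yaw amount.
; On entering the state it picks a target angle between configurable min and max values.
; Each tick it adds local yaw scaled by turn speed and delta time, accumulates the total, and finishes successfully once the target is reached.
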(event EventLatentTick
  (params (DeltaTime :type Float%20%28single-precision%29))
  (CallFunction|Rotate DeltaTime))

(event EventLatentEnterState
  (params (Transition :type State%20Tree%20Transition%20Result%20Structure%20%28by%20ref%29))
  (Variables|Default|SetAccRotation 0.0)
  (Variables|Default|SetRotateAmount (Math|Random|RandomFloatinRange (Variables|Default|GetMinRotateAmount) (Variables|Default|GetMaxRotateAmount))))

(fn Rotate
  (params (DeltaTime :type Float%20%28double-precision%29))
  (bind _output_get (LocalVariables|SetDeltaRotation (* DeltaTime (Variables|Default|GetTurnSpeed))))
  (Transformation|AddActorLocalRotation (Variables|Default|GetActorToRotate) (Math|Rotator|MakeRotator 0.0 0.0 _output_get) false false)
  (bind _output_get_2 (Variables|Default|SetAccRotation (+ (Variables|Default|GetAccRotation) (LocalVariables|GetDeltaRotation))))
  (if (>= _output_get_2 (Variables|Default|GetRotateAmount))
    (StateTree|FinishTask true)))