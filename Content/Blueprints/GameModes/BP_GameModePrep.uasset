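; Game mode for a timed prep phase that loads the next level by name when the countdown runs out.
; BeginPlay records the start time, and remaining time is derived from the phase duration minus elapsed game time.
; Tick polls that value to trigger the level change.
; GetPhaseLabel formats the same value as a minutes-and-seconds "Time:" text.
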(event EventBeginPlay
  (|CallParentFunction)
  (Variables|Default|SetPhaseStart (Utilities|Time|GetGameTimeinSeconds)))

(event EventTick
  (params (DeltaSeconds :type Float%20%28single-precision%29))
  (|CallParentFunction DeltaSeconds)
  (if (<= (CallFunction|GetRemainingPhaseTime) 0.0)
    (Game|OpenLevel(byName) (Variables|Default|GetNextLevelName))))

(fn ConstructionScript
  (|CallParentFunction))

(fn GetPhaseLabel
  (bind _output_get (LocalVariables|SetDeltaTime (Math|Float|Floor (CallFunction|GetRemainingPhaseTime))))
  (return (Utilities|Text|FormatText "Time: {Minutes}:{Seconds}" (Utilities|Text|ToText(Integer) (/ _output_get 60) false true 2) (Utilities|Text|ToText(Integer) (Math|Integer|%(Integer) _output_get 60) false true 2))))

(fn GetRemainingPhaseTime
  (return (- (Variables|Default|GetPhaseDuration) (- (Utilities|Time|GetGameTimeinSeconds) (Variables|Default|GetPhaseStart)))))