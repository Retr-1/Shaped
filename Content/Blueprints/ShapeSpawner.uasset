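; Shape spawner actor that keeps spawning BP_ShapeObject actors at a spawn point, up to a maximum live count.
; A looping cooldown timer drives spawning, stops at the cap and restarts when a spawned shape's destroy event lowers the count.
; Color comes from a weighted roll between wildcard, gray junk and a random regular color.
; GetSpawnedShapeType supplies the shape type, but its random selection node is unused.
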(event Custom|SpawnShapeEvent
  (|SpawnShape))

(event Custom|InitializeSpawnLoop
  (if (not (Class|KismetSystemLibrary|TimerExistsHandle (Variables|Default|GetSpawnLoop)))
    (bind _returnvalue (Utilities|Time|SetTimerbyEvent (delegate Custom|SpawnShapeEvent) (Variables|Default|GetSpawnCooldown) true))
    (Variables|Default|SetSpawnLoop _returnvalue)))

(event EventBeginPlay
  (CallFunction|InitializeSpawnLoop))

(event Collision|EventActorBeginOverlap
  (params (OtherActor :type Actor%20Object%20Reference)))

(event EventTick
  (params (DeltaSeconds :type Float%20%28single-precision%29)))

(fn ConstructionScript)

(fn GetSpawnedShapeColor
  (bind _output_get (LocalVariables|SetRandomFloat (Math|Random|RandomFloat)))
  (if (<= _output_get (Variables|Default|GetWildcardChance))
    (return "Wildcard")
    (elif (<= (LocalVariables|GetRandomFloat) (+ (Variables|Default|GetWildcardChance) (Variables|Default|GetJunkChance)))
      (return "Gray")
      (else
        (return (Utilities|Select :Index (Math|Random|RandomIntegerinRange 0 (- (|GetNumEnumEntries) 2)) :Option%200 "Red" :Option%201 "Green" :Option%202 "Blue" :Option%203 "Yellow"))))))

(event Custom|ShapeDestroyed
  (params (DestroyedActor :type Actor%20Object%20Reference))
  (Variables|Default|SetSpawnedShapesCount (- (Variables|Default|GetSpawnedShapesCount) 1))
  (CallFunction|InitializeSpawnLoop))