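; BP_Base is the base that enemies attack, tracking a Health value that starts at MaxHealth.
; When a BP_EnemyBase actor overlaps its Sphere component, the base subtracts that enemy's DamageToBase and destroys the enemy.
; It then calls OnBaseDamaged with itself as the argument so listeners can react; no death handling happens here.
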(event OnComponentBeginOverlap(Sphere)
  (params (OverlappedComponent :type Primitive%20Component%20Object%20Reference) (OtherActor :type Actor%20Object%20Reference) (OtherComp :type Primitive%20Component%20Object%20Reference) (OtherBodyIndex :type Integer) (bFromSweep :type Boolean) (SweepResult :type Hit%20Result%20Structure%20%28by%20ref%29))
  (bind _asbp_enemy_base (Utilities|Casting|CastToBP_EnemyBase OtherActor))
  (Variables|Default|SetHealth (- (Variables|Default|GetHealth) (Variables|/Game/Blueprints/Enemy/BP_EnemyBase.BP_EnemyBase_C|GetDamageToBase _asbp_enemy_base)))
  (Actor|DestroyActor _asbp_enemy_base)
  (Default|CallOnBaseDamaged self))

(event EventBeginPlay
  (Variables|Default|SetHealth (Variables|Default|GetMaxHealth)))

(event Collision|EventActorBeginOverlap
  (params (OtherActor :type Actor%20Object%20Reference)))

(event EventTick
  (params (DeltaSeconds :type Float%20%28single-precision%29)))

(fn ConstructionScript)