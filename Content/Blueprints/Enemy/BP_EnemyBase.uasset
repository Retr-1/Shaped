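; Base enemy character that runs a StateTree-driven AI controller, fights the player with melee attacks and awards XP to the game instance on death.
; Attack plays a montage, while StartHitPeriod and EndHitPeriod toggle an overlap hitbox that damages the player once per window.
; Highlighting uses custom depth with a stencil value, and the overhead widget turns toward the camera every tick.
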(event OnComponentBeginOverlap(AttackHitCollision)
  (params (OverlappedComponent :type Primitive%20Component%20Object%20Reference) (OtherActor :type Actor%20Object%20Reference) (OtherComp :type Primitive%20Component%20Object%20Reference) (OtherBodyIndex :type Integer) (bFromSweep :type Boolean) (SweepResult :type Hit%20Result%20Structure%20%28by%20ref%29))
  (if (not (Variables|Default|GetAlreadyHitPlayer))
    (bind _asbp_player_character (Utilities|Casting|CastToBP_PlayerCharacter OtherActor))
    (Class|ShapedPlayerCharacter|ApplyDamagetoPlayer _asbp_player_character (Variables|Default|GetDamageToPlayer))
    (Variables|Default|SetAlreadyHitPlayer true)))

(event Custom|DEBUG
  ;[0.15 0.15 0.15 0.5] Debug
  (CallFunction|EquipSword)
  (Animation|PlayAnimMontage "/Game/Characters/Triangleman1/SkeletalMeshes/AM_Attack.AM_Attack" 1.0 "None"))

(event EventBeginPlay
  (bind _mesh (Variables|Character|GetMesh))
  (Rendering|SetCustomDepthStencilValue _mesh 69)
  (Rendering|SetRenderCustomDepth _mesh false)
  (Pawn|SpawnDefaultController)
  (bind _asaic_base (Utilities|Casting|CastToAIC_Base (Pawn|GetController)))
  (Class|BrainComponent|RestartLogic (Variables|/Game/Blueprints/Enemy/AIC_Base.AIC_Base_C|GetStateTreeAI _asaic_base)))

(event EventOnAllHealthLost
  (bind _asbp_shaped_game_instance (Utilities|Casting|CastToBP_ShapedGameInstance (Game|GetGameInstance)))
  (Default|AddXP _asbp_shaped_game_instance (Variables|Default|GetYieldXPAmount))
  (Actor|DestroyActor))

(event EventTick
  (params (DeltaSeconds :type Float%20%28single-precision%29))
  (|ManageOverheadWidgetRotation))

(event EventSetHighlighted
  (params (IsHighlighted :type Boolean))
  (Rendering|SetRenderCustomDepth (Variables|Character|GetMesh) IsHighlighted))

(fn ConstructionScript)

(fn EquipSword
  (Variables|/Script/Engine.SkeletalMeshComponent|SetSkeletalMeshAsset (Variables|Default|GetWeaponMesh) "/Game/Characters/simplesword/SkeletalMeshes/simplesword.simplesword"))

(fn Attack
  (Animation|PlayAnimMontage "/Game/Characters/Triangleman1/SkeletalMeshes/AM_Attack.AM_Attack" 1.0 "None"))

(fn StartHitPeriod
  (Collision|SetCollisionEnabled (Variables|Default|GetAttackHitCollision) "QueryOnly")
  (Variables|Default|SetAlreadyHitPlayer false))

(fn EndHitPeriod
  (Collision|SetCollisionEnabled (Variables|Default|GetAttackHitCollision) "NoCollision"))