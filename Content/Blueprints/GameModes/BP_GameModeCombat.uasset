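; Combat game mode that tracks remaining enemies and ends the fight phase when none are left.
; On BeginPlay it finds the BP_EnemySpawner, binds to its enemy-amount-changed event and copies the starting count.
; When an updated count reaches zero or below, it tells BP_ShapedGameInstance to move from fight to factory.
; GetPhaseLabel formats the stored count as remaining-enemies text.
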(event Custom|UpdateEnemyCount
  (params (Count :type Integer))
  (bind _output_get (Variables|Default|SetEnemyAmount Count))
  (if (<= _output_get 0)
    (bind _asbp_shaped_game_instance (Utilities|Casting|CastToBP_ShapedGameInstance (Game|GetGameInstance)))
    (Default|MovefromFighttoFactory _asbp_shaped_game_instance)))

(event EventBeginPlay
  (|CallParentFunction)
  (bind _returnvalue (Actor|GetActorOfClass "/Game/Blueprints/BP_EnemySpawner.BP_EnemySpawner_C"))
  (EventDispatchers|BindEventtoEnemyAmountChanged _returnvalue (delegate Custom|UpdateEnemyCount))
  (Variables|Default|SetEnemyAmount (Variables|/Game/Blueprints/BP_EnemySpawner.BP_EnemySpawner_C|GetEnemyAmount _returnvalue)))

(event EventTick
  (params (DeltaSeconds :type Float%20%28single-precision%29))
  (|CallParentFunction DeltaSeconds) ; This node is disabled and will not be called.\nDrag off pins to build functionality.
)

(fn ConstructionScript
  (|CallParentFunction))

(fn GetPhaseLabel
  (return (Utilities|Text|FormatText "Remaining Enemies: { }" (Variables|Default|GetEnemyAmount))))