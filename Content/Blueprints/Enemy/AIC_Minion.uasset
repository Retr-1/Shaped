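; AIC_Minion is the AI controller for minion enemies, using AI perception to detect the player character and drive a StateTree.
; When perception gains or loses the player, it sets CanSeePlayer and TargetActor, sends a seen or unseen gameplay-tag event to the StateTree, and prints a debug string.
; While a target is valid, Tick updates DistanceToPlayer from the controlled pawn's location to the target.
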(event OnTargetPerceptionUpdated(AIPerception)
  (params (Actor :type Actor%20Object%20Reference) (Stimulus :type AI%20Stimulus%20Structure))
  (bind _asbp_player_character (Utilities|Casting|CastToBP_PlayerCharacter Actor))
  (if (.bsuccessfullysensed Stimulus)
    (Variables|Default|SetCanSeePlayer true)
    (Variables|Default|SetTargetActor _asbp_player_character)
    (Gameplay|StateTree|SendStateTreeEvent (Variables|Default|GetStateTreeAI) (Utilities|Struct|MakeStateTreeEvent "(TagName=\"AI.PlayerSeen\")" "None" "None") :!class /Script/GameplayStateTreeModule.StateTreeComponent)
    (Development|PrintString "SEen")
    (else
      (Variables|Default|SetCanSeePlayer false)
      (Variables|Default|SetTargetActor 0)
      (Gameplay|StateTree|SendStateTreeEvent (Variables|Default|GetStateTreeAI) (Utilities|Struct|MakeStateTreeEvent "(TagName=\"AI.PlayerUnseen\")" "None" "None") :!class /Script/GameplayStateTreeModule.StateTreeComponent)
      (Development|PrintString "Unseen"))))

(event EventBeginPlay
  (|CallParentFunction) ; This node is disabled and will not be called.\nDrag off pins to build functionality.
)

(event EventTick
  (params (DeltaSeconds :type Float%20%28single-precision%29))
  (|CallParentFunction DeltaSeconds)
  (Utilities|IsValid (Variables|Default|GetTargetActor)
    (:Is%20Valid
      (Variables|Default|SetDistanceToPlayer (Math|Vector|Distance(Vector) (Transformation|GetActorLocation (Pawn|GetControlledPawn)) (Transformation|GetActorLocation (Variables|Default|GetTargetActor)))))))

(fn ConstructionScript
  (|CallParentFunction))