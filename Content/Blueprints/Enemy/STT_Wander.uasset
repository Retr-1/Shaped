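; StateTree task for enemy wandering that moves the owning pawn to a random reachable point within a radius of its current location.
; On arrival it waits on a timer and then finishes as succeeded, while a failed move finishes the task as failed.
; If the actor is not a Pawn it only prints a debug string and never finishes the task.
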(event EventLatentEnterState
  (params (Transition :type State%20Tree%20Transition%20Result%20Structure%20%28by%20ref%29))
  (|CallParentFunction Transition)
  (bind _aspawn (Utilities|Casting|CastToPawn (Variables|Default|GetActor))
    (:then
      (Development|PrintString "fawefawefawef")
      (AI|AIMoveTo _aspawn (.RandomLocation (AI|Navigation|GetRandomReachablePointinRadius (Transformation|GetActorLocation _aspawn) (Variables|Default|GetRadius) 0 0)) 0 5.0 false
        (:OnSuccess
          (Utilities|Time|SetTimerbyFunctionName 0 "EndWait" (Variables|Default|GetWaitTime)))
        (:OnFail
          (StateTree|FinishTask false))))
    (:CastFailed
      (Development|PrintString "PICEEEEEEEEEE"))))

(fn EndWait
  (StateTree|FinishTask true))