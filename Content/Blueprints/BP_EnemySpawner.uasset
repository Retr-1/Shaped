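; Enemy spawner that, on BeginPlay, spawns a wave sized by the game instance's Cycle.
; A self-calling SpawnEnemy event with a delay places weighted-random enemy types in a half-ring around the spawner.
; Each enemy gets a letter-coded ammo requirement chosen by Cycle stage, starting with a fixed code.
; Enemy destruction events decrement the live count, which is broadcast through EnemyAmountChanged.
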(event Custom|SpawnEnemy
  (if (> (Variables|Default|GetSpawnEnemyAmount) 0)
    (Variables|Default|SetSpawnEnemyAmount (- (Variables|Default|GetSpawnEnemyAmount) 1))
    (bind _returnvalue (Game|SpawnActorfromClass (CallFunction|GetEnemyType) (Math|Transform|MakeTransform (CallFunction|GetRandomSpawnPoint) "0, 0, 0" "1.000000,1.000000,1.000000") "AdjustIfPossibleButAlwaysSpawn" "MultiplyWithRoot" 0 0))
    (Game|BindEventtoOnDestroyed _returnvalue (delegate Custom|DecreaseEnemyAmount))
    (Default|SetAmmoRequirement _returnvalue (CallFunction|GetRandomAmmoRequirement))
    (Development|PrintString "Spawned")
    (Utilities|FlowControl|Delay (Variables|Default|GetSpawnDelay))
    (CallFunction|SpawnEnemy)))

(event Custom|DecreaseEnemyAmount
  (params (DestroyedActor :type Actor%20Object%20Reference))
  (bind _output_get (Variables|Default|SetEnemyAmount (- (Variables|Default|GetEnemyAmount) 1)))
  (Default|CallEnemyAmountChanged _output_get))

(event EventBeginPlay
  (bind _asbp_shaped_game_instance (Utilities|Casting|CastToBP_ShapedGameInstance (Game|GetGameInstance)))
  (bind _output_get (Variables|Default|SetGameInstance _asbp_shaped_game_instance))
  (Variables|Default|SetCycle (Variables|/Game/Blueprints/BP_ShapedGameInstance.BP_ShapedGameInstance_C|GetCycle _output_get))
  (Variables|Default|SetBaseLocation (Transformation|GetActorLocation))
  (CallFunction|SpawnEnemies))

(event Collision|EventActorBeginOverlap
  (params (OtherActor :type Actor%20Object%20Reference)))

(event EventTick
  (params (DeltaSeconds :type Float%20%28single-precision%29)))

(fn ConstructionScript)

(fn GetStartingEnemyAmount
  (return (+ (/ (Variables|Default|GetCycle) 2) 1)))

(fn SpawnEnemies
  (bind _output_get (Variables|Default|SetEnemyAmount (CallFunction|GetStartingEnemyAmount)))
  (Variables|Default|SetSpawnEnemyAmount _output_get)
  (CallFunction|SpawnEnemy)
  (Default|CallEnemyAmountChanged (Variables|Default|GetEnemyAmount)))

(fn GetEnemyType
  (bind _output_get (LocalVariables|SetRandomFloat (Math|Random|RandomFloat)))
  (if (< _output_get 0.4)
    (return "/Game/Blueprints/Enemy/BP_EnemyPrimitive.BP_EnemyPrimitive_C")
    (elif (< (LocalVariables|GetRandomFloat) 0.8)
      (return "/Game/Blueprints/Enemy/BP_EnemyMinion.BP_EnemyMinion_C")
      (else
        (return "/Game/Blueprints/Enemy/BP_EnemyRedLightGreenLight.BP_EnemyRedLightGreenLight_C")))))

(fn GetRandomSpawnPoint
  (bind _baselocation (Variables|Default|GetBaseLocation))
  (LocalVariables|SetRandomR (Math|Random|RandomFloatinRange (Variables|Default|GetMinSpawnR) (Variables|Default|GetMaxSpawnR)))
  (LocalVariables|SetRandomAngle (Math|Random|RandomFloatinRange 0.0 3.1415))
  (return (Math|Vector|MakeVector (+ (.x _baselocation) (* (Math|Trig|Cos(Radians) (LocalVariables|GetRandomAngle)) (LocalVariables|GetRandomR))) (+ (.y _baselocation) (* (LocalVariables|GetRandomR) (Math|Trig|Sin(Radians) (LocalVariables|GetRandomAngle)))) (+ (.z _baselocation) 1e+02))))

(fn GetRandomAmmoRequirement
  (if (< (Variables|Default|GetCycle) 5)
    (return (Utilities|Array|MakeArray "www"))
    (elif (< (Variables|Default|GetCycle) 10)
      (return (|SecondStage))
      (else
        (return (|ThirdStage))))))